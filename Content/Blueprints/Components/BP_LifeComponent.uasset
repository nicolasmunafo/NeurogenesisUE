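; Actor component that tracks a health pool for its owner and triggers death when it runs out.
; CurrentHP starts at MaxHP on BeginPlay, then ReduceLife and IncreaseLife adjust it, clamped between zero and MaxHP.
; When damage brings it to zero, the owner is cast to BP_IKillableActor and Die is called, so only killable owners respond.
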(event `self.ReceiveBeginPlay`
  (set `self.CurrentHP` (`self.MaxHP`)))

(event `ReduceLife`
  (params (ReducedHP :type "Float (double-precision)"))
  (bind _returnvalue (- (`self.CurrentHP`) ReducedHP))
  (if (<= _returnvalue 0.0)
    (set `self.CurrentHP` 0.0)
    (bind _asbp_ikillable_actor (cast `/Game/Blueprints/BP_IKillableActor` (`self.GetOwner`))) ; Check if the owning actor is killable
    (`/Game/Blueprints/BP_IKillableActor.Die` _asbp_ikillable_actor) ; Every killable actor dies if their life\nis set to 0
    (else
      (set `self.CurrentHP` _returnvalue))))

(event `IncreaseLife`
  (params (IncreasedHP :type "Float (double-precision)"))
  (bind _returnvalue (+ IncreasedHP (`self.CurrentHP`)))
  (if (>= _returnvalue (`self.MaxHP`))
    (set `self.CurrentHP` (`self.MaxHP`))
    (else
      (set `self.CurrentHP` _returnvalue))))