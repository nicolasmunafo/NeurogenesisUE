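; AI controller for the boss that starts its blackboard and behavior tree on BeginPlay.
; Perception updates toggle the detected-player key for actors castable to BP_ICharacters, clearing it if already valid rather than checking whether each was sensed or lost.
; Events write awake, phase, sticky-bomb count and death state to the blackboard.
; GetActiveCharacter returns the active character stored there as an Actor.
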(event `self.ReceiveBeginPlay`
  ;[1 1 1] At the start, use blackboard and behavior tree
  (`self.UseBlackboard` "/Game/Blueprints/Boss/BP_BossBlackboard.BP_BossBlackboard")
  (`self.RunBehaviorTree` "/Game/Blueprints/Boss/BP_BossBTree.BP_BossBTree"))

(event `self.AIPerception.OnPerceptionUpdated`
  (params (UpdatedActors :type "Array of Actor Object Reference (by ref)"))
  ;[1 1 1] When a character is detected it will set the blackboard value, if the perception changed it is because no character was detected
  (for _array_element UpdatedActors
    (bind _asbp_icharacters (cast `/Game/Blueprints/Characters/BP_ICharacters` _array_element))
    (`/Engine/EditorBlueprintResources/StandardMacros.IsValid` (`BlackboardComponent.GetValueAsObject` (`AIBlueprintHelperLibrary.GetBlackboard` self) (`self.BossDetectsPlayer`))
      (:`Is Valid`
        (`BlackboardComponent.ClearValue` (`AIBlueprintHelperLibrary.GetBlackboard` self) (`self.BossDetectsPlayer`)))
      (:`Is Not Valid`
        (`BlackboardComponent.SetValueAsObject` (`AIBlueprintHelperLibrary.GetBlackboard` self) (`self.BossDetectsPlayer`) (`KismetSystemLibrary.Conv_InterfaceToObject` _asbp_icharacters))))))

(event `ChangeAwakeState`
  (`BlackboardComponent.SetValueAsBool` (`AIBlueprintHelperLibrary.GetBlackboard` self) (`self.BBAwake`) true) ; If it was not awake, set IsAwake to true
)

(event `IncrementBombs`
  (bind _returnvalue (`AIBlueprintHelperLibrary.GetBlackboard` self))
  (`BlackboardComponent.SetValueAsInt` _returnvalue (`self.BBStickyBomb`) (+ (`BlackboardComponent.GetValueAsInt` _returnvalue (`self.BBStickyBomb`)) 1)))

(event `DecrementBombs`
  (bind _returnvalue (`AIBlueprintHelperLibrary.GetBlackboard` self))
  (`BlackboardComponent.SetValueAsInt` _returnvalue (`self.BBStickyBomb`) (- (`BlackboardComponent.GetValueAsInt` _returnvalue (`self.BBStickyBomb`)) 1)))

(event `ChangeToPhase`
  (params (NewPhaseNum :type Integer))
  (`BlackboardComponent.SetValueAsInt` (`AIBlueprintHelperLibrary.GetBlackboard` self) (`self.BBPhaseNumber`) NewPhaseNum))

(event `BossIsDead`
  (`BlackboardComponent.SetValueAsBool` (`AIBlueprintHelperLibrary.GetBlackboard` self) (`self.BBBossDead`) true))

(fn `GetActiveCharacter`
  (returns (ActiveCharacter :type "Actor Object Reference"))
  (bind _asactor (cast `Actor` (`BlackboardComponent.GetValueAsObject` (`AIBlueprintHelperLibrary.GetBlackboard` self) (`self.BBActiveChar`))))
  (return _asactor))

(fn `UserConstructionScript`)