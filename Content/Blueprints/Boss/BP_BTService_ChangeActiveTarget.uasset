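; Behavior tree service for the boss that switches which player character is its active target.
; On each AI tick it reads the bomb count from the Blackboard.
; With at least one bomb it writes the secondary character to the active-character key, otherwise the main character, each found by class lookup.
; A duplicate copy of this logic sits unconnected and never runs.
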(event `self.ReceiveSearchStartAI`
  (params (OwnerController :type "AIController Object Reference") (ControlledPawn :type "Pawn Object Reference")))

(event `self.ReceiveTickAI`
  (params (OwnerController :type "AIController Object Reference") (ControlledPawn :type "Pawn Object Reference") (DeltaSeconds :type "Float (single-precision)"))
  (bind _returnvalue (`AIBlueprintHelperLibrary.GetBlackboard` OwnerController))
  (bind _bbactivechar (`self.BBActiveChar`))
  (if (>= (`BlackboardComponent.GetValueAsInt` _returnvalue (`self.BBBombsNum`)) 1)
    (bind _returnvalue_2 (`GameplayStatics.GetActorOfClass` "/Game/Blueprints/Characters/BP_SecondaryCharacter.BP_SecondaryCharacter_C")) ; If there is at least a bomb, attack second character
    (`BlackboardComponent.SetValueAsObject` _returnvalue _bbactivechar _returnvalue_2)
    (else
      (bind _returnvalue_3 (`GameplayStatics.GetActorOfClass` "/Game/Blueprints/Characters/BP_MainCharacter.BP_MainCharacter_C"))
      (`BlackboardComponent.SetValueAsObject` _returnvalue _bbactivechar _returnvalue_3))))