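; Behavior tree decorator for the boss that gates its first-phase attack.
; The AI condition check reads the phase number from the blackboard and passes only when it equals 1.
; Leftover disconnected logic, which never runs, would set the active character target to the secondary character while bombs remain and to the main character otherwise.
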(event `self.ReceiveObserverActivatedAI`
  (params (OwnerController :type "AIController Object Reference") (ControlledPawn :type "Pawn Object Reference")))

(fn `PerformConditionCheckAI`
  (params (OwnerController :type "AIController Object Reference") (ControlledPawn :type "Pawn Object Reference"))
  (returns (ReturnValue :type Boolean))
  (if (== (`BlackboardComponent.GetValueAsInt` (`AIBlueprintHelperLibrary.GetBlackboard` OwnerController) (`self.BBPhaseNum`)) 1)
    (return true)
    (else
      (return false))))