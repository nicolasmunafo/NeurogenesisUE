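; Behavior tree decorator for the boss that passes when the blackboard bomb count is at least one.
; On a pass it copies that count to the previous-count key, stores the first found BP_SecondaryCharacter as the active character and prints a debug message.
; Despite the name, it never tests for an increase: the comparison against the previous count is disconnected, and the observer activation event is empty.
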(event `self.ReceiveObserverActivatedAI`
  (params (OwnerController :type "AIController Object Reference") (ControlledPawn :type "Pawn Object Reference")))

(fn `PerformConditionCheckAI`
  (params (OwnerController :type "AIController Object Reference") (ControlledPawn :type "Pawn Object Reference"))
  (returns (ReturnValue :type Boolean))
  (bind _returnvalue (`AIBlueprintHelperLibrary.GetBlackboard` OwnerController))
  (bind _returnvalue_2 (`BlackboardComponent.GetValueAsInt` (`AIBlueprintHelperLibrary.GetBlackboard` OwnerController) (`self.BBSBombNum`)))
  (if (>= _returnvalue_2 1)
    (`BlackboardComponent.SetValueAsInt` _returnvalue (`self.BBSPreviousBombNum`) _returnvalue_2)
    (bind _returnvalue_3 (`GameplayStatics.GetActorOfClass` "/Game/Blueprints/Characters/BP_SecondaryCharacter.BP_SecondaryCharacter_C"))
    (`BlackboardComponent.SetValueAsObject` _returnvalue (`self.BBActiveChar`) _returnvalue_3)
    (`KismetSystemLibrary.PrintString` "Has a Bomb!!")
    (return true)))