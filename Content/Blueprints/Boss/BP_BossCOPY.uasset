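; Boss actor that spins every tick, fires a mouth beam and reports its death to BP_GameManager.
; BossFire animates the mouth material colour through timelines, then after a delay spawns the beam emitter and sphere-traces along RayOrigin to damage what it hits.
; Patrol adds timeline-driven yaw and FlipAround turns BossDirection.
; Player-facing logic is disconnected; watch, focused attack and death display are stubs.
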(event `BossRay`
  (bind _rayorigin (`self.RayOrigin`))
  (bind _returnvalue (`GameplayStatics.SpawnEmitterAtLocation` "/Game/Materials/LaserBeam/BossBeam.BossBeam" (`SceneComponent.K2_GetComponentLocation` _rayorigin) (`KismetMathLibrary.Conv_VectorToRotator` (`SceneComponent.GetUpVector` _rayorigin)) (20.0 20.0 20.0)))
  (`KismetSystemLibrary.Delay` 0.4)
  (`KismetSystemLibrary.PrintString` "spawn")
  (`ActorComponent.K2_DestroyComponent` _returnvalue))

(event `BossFocusedAttack`
  (`KismetSystemLibrary.PrintString` "Focused Attack" true true (struct :`R` 1.0 :`G` 0.025978 :`A` 1.0)))

(event `BossFire`
  (bind (_direction _colorchange) (`Timeline|Color`)
    (:`Update`
      (bind _returnvalue (`PrimitiveComponent.CreateDynamicMaterialInstance` (`self.BossFace`) 0 "/Game/Materials/Boss/boca.boca" "None"))
      (`MaterialInstanceDynamic.SetVectorParameterValue` _returnvalue "MouthColor" _colorchange)
      (`KismetSystemLibrary.Delay` 2.0)
      (`self.BossRay`)
      (`self.FireMouth`)
      (bind _returnvalue_2 (`PrimitiveComponent.CreateDynamicMaterialInstance` (`self.BossFace`) 0 "/Game/Materials/Boss/boca.boca" "None"))
      (bind (_direction_2 _colorchange_2) (`Timeline|Timeline_0`)
        (:`Update`
          (`MaterialInstanceDynamic.SetVectorParameterValue` _returnvalue_2 "MouthColor" _colorchange_2)
          (`KismetSystemLibrary.Delay` 2.0))))))

(event `BossPatrol`
  (bind (_direction _newtrack_0) (`Timeline|Rotator` :!label _label)
    (:`Update`
      (`self.K2_AddActorLocalRotation` (`KismetMathLibrary.MakeRotator` 0.0 0.0 _newtrack_0)))))

(event `BossStopPatrol`
  (goto _label :!via `Stop`))

(event `BossWatch`)

(event `self.ReceiveTick`
  (params (DeltaSeconds :type "Float (single-precision)"))
  (`self.K2_AddActorLocalRotation` (struct :`Yaw` 1.0)))

(event `FlipAround`
  (bind _bossdirection (`self.BossDirection`))
  (bind (_returnvalue_roll _returnvalue_pitch) (`KismetMathLibrary.BreakRotator` (`SceneComponent.K2_GetComponentRotation` _bossdirection)))
  (bind _returnvalue_location (`KismetMathLibrary.BreakTransform` (`SceneComponent.GetRelativeTransform` (`self.BossDirection`))))
  (set `self.HasFlipped` true)
  (`KismetSystemLibrary.MoveComponentTo` _bossdirection _returnvalue_location (`KismetMathLibrary.MakeRotator` _returnvalue_roll _returnvalue_pitch 180.0) false false 1.0))

(event `RestoreWatch`
  (set `self.HasFlipped` false))

(event `/Game/Blueprints/BP_IKillableActor.Die`
  ;[1 1 1] When the boss dies, it will inform the GameManager
  (`self.ShowDeath`)
  (bind _returnvalue (`GameplayStatics.GetActorOfClass` "/Game/Blueprints/GameManagers/BP_GameManager.BP_GameManager_C"))
  (`/Game/Blueprints/GameManagers/BP_GameManager.BossHasDied` _returnvalue))

(fn `FireMouth`
  (bind _rayorigin (`self.RayOrigin`))
  (bind _returnvalue (`SceneComponent.K2_GetComponentLocation` _rayorigin))
  (bind (_outhit _returnvalue_2) (`KismetSystemLibrary.SphereTraceSingle` :`Start` _returnvalue :`End` (+ _returnvalue (* (`SceneComponent.GetUpVector` _rayorigin) 20000.0)) :`Radius` 30.0 :`TraceChannel` "TraceTypeQuery5" :`DrawDebugType` "ForOneFrame" :`DrawTime` 1.0))
  (if _returnvalue_2
    (message `/Game/Blueprints/Characters/BP_ICharacters.BeAttackedByEnemy` (`.HitActor` (`GameplayStatics.BreakHitResult` _outhit)) (`/Game/Blueprints/Components/BP_DamageComponent.DamagePoints` (`self.BP_DamageComponent`)))))

(fn `Flip`
  (params (InitalRotation :type "Rotator Structure"))
  (`self.K2_SetActorRelativeRotation` InitalRotation))

(fn `ShowDeath`)

(fn `UserConstructionScript`)