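; Boss character that sleeps until hit by a sticky bomb, which wakes it into phase 1 and closes level doors.
; It reports bomb counts, phase two at low health, and death to BP_BossAIController; death also notifies the GameManager.
; Timelines drive patrol spin, aiming and mouth color, with firing using a delayed sphere trace and beam particle to damage characters.
; It also exposes an event that triggers enemy spawners for phase two.
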(event `BossRay`
  (bind _rayorigin (`self.RayOrigin`))
  ;[1 1 1] Spawn ray emitter
  (bind _returnvalue (`GameplayStatics.SpawnEmitterAtLocation` "/Game/Materials/LaserBeam/BossBeam.BossBeam" (`SceneComponent.K2_GetComponentLocation` _rayorigin) (`KismetMathLibrary.Conv_VectorToRotator` (`SceneComponent.GetUpVector` _rayorigin)) (20.0 20.0 20.0)))
  (`KismetSystemLibrary.Delay` 0.4)
  (`ActorComponent.K2_DestroyComponent` _returnvalue))

(event `BossFire`
  ;[1 1 1] Shoot ray to damage character
  (bind (_direction _colorchange) (`Timeline|Color`)
    (:`Update`
      (bind _returnvalue (`PrimitiveComponent.CreateDynamicMaterialInstance` (`self.BossFace`) 0 "/Game/Materials/Boss/boca.boca" "None"))
      (`MaterialInstanceDynamic.SetVectorParameterValue` _returnvalue "MouthColor" _colorchange)
      (`KismetSystemLibrary.Delay` (`self.ShootingDelay`))
      (`GameplayStatics.PlaySoundAtLocation` "/Game/Audio/Boss/369516__kinoton__energy-blast_-_BOSS_SHOOT.369516__kinoton__energy-blast_-_BOSS_SHOOT" (`self.K2_GetActorLocation`) (struct) 1.0 1.0 0.0 "/Game/Audio/SoundAttenuationBoss.SoundAttenuationBoss" null null)
      (`self.FireMouth`)
      (`self.BossRay`)
      (bind _returnvalue_2 (`PrimitiveComponent.CreateDynamicMaterialInstance` (`self.BossFace`) 0 "/Game/Materials/Boss/boca.boca" "None"))
      (bind (_direction_2 _colorchange_2) (`Timeline|Timeline_0`)
        (:`Update`
          (`MaterialInstanceDynamic.SetVectorParameterValue` _returnvalue_2 "MouthColor" _colorchange_2))))))

(event `/Game/Blueprints/BP_IKillableActor.Die`
  ;[1 1 1] When the boss dies, it will inform the GameManager
  (`self.ShowDeath`)
  (bind _returnvalue (`GameplayStatics.GetActorOfClass` "/Game/Blueprints/GameManagers/BP_GameManager.BP_GameManager_C"))
  (`/Game/Blueprints/GameManagers/BP_GameManager.BossHasDied` _returnvalue))

(event `self.ReceiveBeginPlay`
  ;[1 1 1] Store the controller blackboard for future references
  (set `self.ControllerBlackBoard` (`AIBlueprintHelperLibrary.GetBlackboard` (`AIBlueprintHelperLibrary.GetAIController` self))))

(event `GotStickyBomb`
  (bind _asbp_boss_aicontroller (cast `/Game/Blueprints/Boss/BP_BossAIController` (`self.GetController`) :!pure true))
  ;[1 1 1] If it got a sticky bomb, increment the number of bombs (if it was sleep, awake)
  (if (not (`BlackboardComponent.GetValueAsBool` (`self.ControllerBlackBoard`) (`self.BBAwake`)))
    (`/Game/Blueprints/Boss/BP_BossAIController.ChangeAwakeState` _asbp_boss_aicontroller)
    (`/Game/Blueprints/Boss/BP_BossAIController.ChangeToPhase` _asbp_boss_aicontroller 1)
    (`PrimitiveComponent.SetMaterial` (`self.BossFace`) 0 "/Game/Materials/Boss/boca.boca")
    (`PrimitiveComponent.SetMaterial` (`self.BossFace`) 4 "/Game/Materials/Boss/ojos.ojos")
    (bind _outactors (`GameplayStatics.GetAllActorsOfClass` "/Game/Blueprints/Switches/BP_DoorClosedOnTrigger.BP_DoorClosedOnTrigger_C"))
    (for _array_element _outactors
      (`/Game/Blueprints/Switches/BP_DoorClosedOnTrigger.CloseDoor` _array_element)))
  (`/Game/Blueprints/Boss/BP_BossAIController.IncrementBombs` (cast `/Game/Blueprints/Boss/BP_BossAIController` (`self.GetController`) :!pure true)))

(event `BombHasExploded`
  ;[1 1 1] If a bomb has exploded, decrement the number of bombs
  (`/Game/Blueprints/Boss/BP_BossAIController.DecrementBombs` (cast `/Game/Blueprints/Boss/BP_BossAIController` (`self.GetController`) :!pure true))
  (`self.CheckSecondPhase`))

(event `RotateToLookAt`
  (params (TargetCharacterPosition :type "Vector Structure"))
  (bind _returnvalue (`self.K2_GetActorRotation`))
  ;[1 1 1] Rotate while shooting
  (set `self.RayInitialRotation` (`SceneComponent.K2_GetComponentRotation` (`self.RayOrigin`)))
  (set `self.InitalRotation` _returnvalue)
  (bind (_direction _rotationcurve) (`Timeline|BossRotationLerp` :!via `PlayFromStart`)
    (:`Update`
      (`self.K2_SetActorRotation` (`KismetMathLibrary.MakeRotator` (.roll _returnvalue) (.pitch _returnvalue) (.yaw (`KismetMathLibrary.RLerp` (`self.InitalRotation`) (`KismetMathLibrary.FindLookAtRotation` (`self.K2_GetActorLocation`) TargetCharacterPosition) _rotationcurve true))))
      (`SceneComponent.K2_SetWorldRotation` (`self.RayOrigin`) (`KismetMathLibrary.RLerp` (`self.RayInitialRotation`) (`KismetMathLibrary.MakeRotFromZ` (`KismetMathLibrary.Normal` (- TargetCharacterPosition (`SceneComponent.K2_GetComponentLocation` (`self.RayOrigin`))))) _rotationcurve) false false)
      (`self.BossFire`))))

(event `StartSpawningEnemies`
  ;[1 1 1] Start spawning enemies during phase 2
  (for _array_element (`self.EnemySpawnerArray`)
    (`/Game/Blueprints/GameManagers/BP_EnemySpawner.Spawn Enemies` _array_element)))

(event `self.ReceiveTick`
  (params (DeltaSeconds :type "Float (single-precision)")))

(event `BossPatrol`
  (bind (_direction _newtrack_0) (`Timeline|Rotator` :!label _label)
    (:`Update`
      (`self.K2_AddActorLocalRotation` (`KismetMathLibrary.MakeRotator` 0.0 0.0 _newtrack_0)))))

(event `BossStopPatrol`
  (goto _label :!via `Stop`))

(event `BossWatch`)

(event `FlipAround`
  (bind _bossdirection (`self.BossDirection`))
  (bind (_returnvalue_roll _returnvalue_pitch) (`KismetMathLibrary.BreakRotator` (`SceneComponent.K2_GetComponentRotation` _bossdirection)))
  (bind _returnvalue_location (`KismetMathLibrary.BreakTransform` (`SceneComponent.GetRelativeTransform` (`self.BossDirection`))))
  (set `self.HasFlipped` true)
  (`KismetSystemLibrary.MoveComponentTo` _bossdirection _returnvalue_location (`KismetMathLibrary.MakeRotator` _returnvalue_roll _returnvalue_pitch 180.0) false false 1.0))

(event `RestoreWatch`
  (set `self.HasFlipped` false))

(event `BossFocusedAttack`
  (`KismetSystemLibrary.PrintString` "Focused Attack" true true (struct :`R` 1.0 :`G` 0.025978 :`A` 1.0)))

(fn `CheckSecondPhase`
  (bind _bp_lifecomponent (`self.BP_LifeComponent`))
  (bind _currenthp (`/Game/Blueprints/Components/BP_LifeComponent.CurrentHP` _bp_lifecomponent))
  (bind _returnvalue (* (`/Game/Blueprints/Components/BP_LifeComponent.MaxHP` _bp_lifecomponent) (`self.LifeThresholdPercPhase2`)))
  ;[1 1 1] If life<=Maxlife * (threshold percentage) => go to phase 2
  (`KismetSystemLibrary.PrintString` (`KismetStringLibrary.Concat_StrStr` "Current" (`KismetStringLibrary.Conv_DoubleToString` _currenthp) "Percentage" (`KismetStringLibrary.Conv_DoubleToString` _returnvalue)))
  (if (<= _currenthp _returnvalue)
    (`/Game/Blueprints/Boss/BP_BossAIController.ChangeToPhase` (cast `/Game/Blueprints/Boss/BP_BossAIController` (`self.GetController`) :!pure true) 2)))

(fn `FireMouth`
  (bind _rayorigin (`self.RayOrigin`))
  (bind _returnvalue (`SceneComponent.K2_GetComponentLocation` _rayorigin))
  (bind (_outhit _returnvalue_2) (`KismetSystemLibrary.SphereTraceSingle` :`Start` _returnvalue :`End` (+ _returnvalue (* (`SceneComponent.GetUpVector` _rayorigin) 20000.0)) :`Radius` 30.0 :`TraceChannel` "TraceTypeQuery5" :`DrawTime` 1.0))
  (if _returnvalue_2
    (bind _asbp_icharacters (cast `/Game/Blueprints/Characters/BP_ICharacters` (`.HitActor` (`GameplayStatics.BreakHitResult` _outhit))))
    (`/Game/Blueprints/Characters/BP_MainCharacter.BeAttackedByEnemy` _asbp_icharacters (`/Game/Blueprints/Components/BP_DamageComponent.DamagePoints` (`self.BP_DamageComponent`)))))

(fn `Flip`
  (params (InitalRotation :type "Rotator Structure"))
  (`self.K2_SetActorRelativeRotation` InitalRotation))

(fn `RotateToEnemy`
  (bind _asactor (cast `Actor` (`BlackboardComponent.GetValueAsObject` (`self.ControllerBlackBoard`) (`self.BBActiveChar`))))
  (bind (_returnvalue_roll _returnvalue_pitch _returnvalue_yaw) (`KismetMathLibrary.BreakRotator` (`KismetMathLibrary.MakeRotFromZ` (`KismetMathLibrary.Normal` (- (`self.K2_GetActorLocation` _asactor) (`SceneComponent.K2_GetComponentLocation` (`self.RayOrigin`)))))))
  (`SceneComponent.K2_SetWorldRotation` (`self.RayOrigin`) (`KismetMathLibrary.MakeRotator` _returnvalue_roll _returnvalue_pitch _returnvalue_yaw) false false))

(fn `ShowDeath`
  (`/Game/Blueprints/Boss/BP_BossAIController.BossIsDead` (cast `/Game/Blueprints/Boss/BP_BossAIController` (`self.GetController`) :!pure true)))

(fn `UserConstructionScript`)