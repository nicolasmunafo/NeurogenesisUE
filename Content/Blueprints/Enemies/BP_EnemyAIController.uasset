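; AI controller for enemies that starts their blackboard and behavior tree on BeginPlay.
; On perception updates, each actor implementing BP_ICharacters toggles the detected-player blackboard key: an existing valid value is cleared, otherwise the actor is stored.
; Storing a target also calls ChaseCharacters on the controlled BP_Enemy.
; Loss of sight is inferred from that toggle rather than read from the stimulus.
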(event `self.ReceiveBeginPlay`
  (`self.UseBlackboard` "/Game/Blueprints/Enemies/BP_EnemyBlackBoard.BP_EnemyBlackBoard")
  (`self.RunBehaviorTree` "/Game/Blueprints/Enemies/BP_EnemyBTree.BP_EnemyBTree"))

(event `self.ReceiveTick`
  (params (DeltaSeconds :type "Float (single-precision)")))

(event `self.AIPerception.OnPerceptionUpdated`
  (params (UpdatedActors :type "Array of Actor Object Reference (by ref)"))
  (for _array_element UpdatedActors
    (bind _asbp_icharacters (cast `/Game/Blueprints/Characters/BP_ICharacters` _array_element)) ; Check if one of the actors implements the\ninterface ICharacters
    (`/Engine/EditorBlueprintResources/StandardMacros.IsValid` (`BlackboardComponent.GetValueAsObject` (`AIBlueprintHelperLibrary.GetBlackboard` self) (`self.BB_DetectedPlayerName`)) ; If the character is valid, then it is because it was\npreviously detected correctly, then it should be\ncleared\nIf the character is not valid, then the player has been \nperceived
      (:`Is Valid`
        (`BlackboardComponent.ClearValue` (`AIBlueprintHelperLibrary.GetBlackboard` self) (`self.BB_DetectedPlayerName`)))
      (:`Is Not Valid`
        (`BlackboardComponent.SetValueAsObject` (`AIBlueprintHelperLibrary.GetBlackboard` self) (`self.BB_DetectedPlayerName`) (`KismetSystemLibrary.Conv_InterfaceToObject` _asbp_icharacters))
        (bind _asbp_enemy (cast `/Game/Blueprints/Enemies/BP_Enemy` (`self.K2_GetPawn`)))
        (`/Game/Blueprints/Enemies/BP_Enemy.ChaseCharacters` _asbp_enemy)))))

(fn `UserConstructionScript`)