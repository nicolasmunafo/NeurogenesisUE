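; Enemy actor that attacks characters, takes their shots and reports its death to BP_GameManager.
; Attacks pass damage component points to the target; shots apply the shooter's damage component to this life component, healing the shooter on a lethal hit or briefly tinting the mesh via dynamic material instances.
; Death plays sound and steam particles, then destroys the actor.
; Other events store patrol waypoints and play a chase sound.
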(event `AttackPlayer`
  (params (CharacterToAttack :type "/Game/Blueprints/Characters/BP_ICharacters Interface"))
  ;[1 1 1] Attacks the character, if it is the second character it will only attack once
  (`/Game/Blueprints/Characters/BP_ICharacters.BeAttackedByEnemy` CharacterToAttack (`/Game/Blueprints/Components/BP_DamageComponent.DamagePoints` (`self.BP_DamageComponent`)))
  (`AudioComponent.Play` (`self.AttackSound`) 0.0))

(event `/Game/Blueprints/BP_IKillableActor.Die`
  (bind _returnvalue (`GameplayStatics.GetActorOfClass` "/Game/Blueprints/GameManagers/BP_GameManager.BP_GameManager_C"))
  (`/Game/Blueprints/GameManagers/BP_GameManager.EnemyHasDied` _returnvalue self)
  (`GameplayStatics.PlaySoundAtLocation` "/Game/Audio/Enemies/182788__robinhood76__04282-demon-passing_-_ENEMY_DEATH.182788__robinhood76__04282-demon-passing_-_ENEMY_DEATH" (`self.K2_GetActorLocation`) (struct) 1.0 1.0 0.0 "/Game/Audio/SoundAttenuationObjects.SoundAttenuationObjects" null null)
  (`AudioComponent.Stop` (`self.AttackSound`))
  (`KismetSystemLibrary.Delay` 0.2)
  (bind _returnvalue_2 (`GameplayStatics.SpawnEmitterAtLocation` "/Game/StarterContent/Particles/P_Steam_Lit.P_Steam_Lit" (`self.K2_GetActorLocation`)))
  (`self.K2_DestroyActor`))

(event `/Game/Blueprints/BP_IShootableActor.GetShotByCharacter`
  (params (Character :type "/Game/Blueprints/Characters/BP_MainCharacter Object Reference"))
  (bind _bp_lifecomponent (`self.BP_LifeComponent`))
  (bind _currenthp (`/Game/Blueprints/Components/BP_LifeComponent.CurrentHP` _bp_lifecomponent))
  (`/Game/Blueprints/Components/BP_DamageComponent.Damage` (`self.GetComponentByClass` Character "/Game/Blueprints/Components/BP_DamageComponent.BP_DamageComponent_C") _bp_lifecomponent)
  (`KismetSystemLibrary.PrintString` (`KismetStringLibrary.Conv_DoubleToString` _currenthp))
  (if (<= _currenthp 0.0)
    (`/Game/Blueprints/Components/BP_LifeComponent.IncreaseLife` (`/Game/Blueprints/Characters/BP_MainCharacter.BP_LifeComponent` Character) (`self.LifeIncreasePerDeath`))
    (else
      (`self.HitColorChange` self)
      (`KismetSystemLibrary.Delay` 0.2)
      (`self.HitColorRestore` self))))

(event `AssignPatrolWaypoints`
  (params (TargetPointsArray :type "Array of TargetPoint Object Reference"))
  (set `self.PatrolWaypoints` TargetPointsArray))

(event `ChaseCharacters`
  (`GameplayStatics.PlaySoundAtLocation` "/Game/Audio/Enemies/395022__alex-dim__horror-creepy-whispering-voice_-_ENEMY_CHASING.395022__alex-dim__horror-creepy-whispering-voice_-_ENEMY_CHASING" (`self.K2_GetActorLocation`) (struct) 1.0 1.0 0.0 "/Game/Audio/SoundAttenuationObjects.SoundAttenuationObjects" null null))

(fn `HitColorChange`
  (bind _returnvalue (`PrimitiveComponent.CreateDynamicMaterialInstance` (`self.Mesh`) 0 "/Game/Mannequin/Character/Materials/CoolUe4ManBody.CoolUe4ManBody" "None"))
  (`MaterialInstanceDynamic.SetVectorParameterValue` _returnvalue "HitColor" (struct :`R` 0.958333 :`G` 0.086637 :`B` 0.666163 :`A` 1.0)))

(fn `HitColorRestore`
  (bind _returnvalue (`PrimitiveComponent.CreateDynamicMaterialInstance` (`self.Mesh`) 0 "/Game/Mannequin/Character/Materials/CoolUe4ManBody.CoolUe4ManBody" "None"))
  (`MaterialInstanceDynamic.SetVectorParameterValue` _returnvalue "HitColor" (struct :`R` 0.181164 :`G` 0.309469 :`B` 0.135633 :`A` 1.0)))

(fn `UserConstructionScript`)