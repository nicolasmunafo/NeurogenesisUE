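; Behavior tree task that picks the next patrol destination for a BP_Enemy.
; On execute it selects a random actor from the enemy's PatrolWaypoints, writes that actor's location to the DestinationBBName blackboard key and finishes with success.
; The pick can repeat the current waypoint, and a pawn that fails the BP_Enemy cast leaves the task without a FinishExecute call.
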(event `self.ReceiveExecuteAI`
  (params (OwnerController :type "AIController Object Reference") (ControlledPawn :type "Pawn Object Reference"))
  (bind _asbp_enemy (cast `/Game/Blueprints/Enemies/BP_Enemy` ControlledPawn))
  (bind _patrolwaypoints (`/Game/Blueprints/Enemies/BP_Enemy.PatrolWaypoints` _asbp_enemy))
  (`BlackboardComponent.SetValueAsVector` (`AIBlueprintHelperLibrary.GetBlackboard` OwnerController) (`self.DestinationBBName`) (`Actor.K2_GetActorLocation` (`|GetArrayItem` _patrolwaypoints (`KismetMathLibrary.RandomIntegerInRange` 0 (- (`KismetArrayLibrary.Array_Length` _patrolwaypoints) 1)))))
  (`self.FinishExecute` true))