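; Game manager actor that runs level flow: soundtrack, pause menu, player death, boss victory and tutorial hints.
; Death events unpossess the player and show BP_MainHUD screens; boss death also destroys all enemies and later opens StartScreen.
; One-shot trigger volumes show timed hints on BP_MainCharacter or BP_SecondaryCharacter, with two more event-driven hints for Axon's death and revival.
; Pit logic is unfinished: enemy deaths inside it are counted without effect.
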(event `self.ReceiveBeginPlay`
  (if (not (`self.IsStartScreen`))
    (`WidgetBlueprintLibrary.SetInputMode_GameOnly` (`GameplayStatics.GetPlayerController` 0)) ; Focuses the cursor again in the viewport
  )
  (`AudioMixerBlueprintLibrary.PrimeSoundCueForPlayback` "/Game/Blueprints/SoundTrack.SoundTrack")
  (`GameplayStatics.PlaySound2D` "/Game/Blueprints/SoundTrack.SoundTrack" 1.0 1.0 0.0 null null))

(event `PlayerHasDied`
  ;[1 1 1] Manage player death
  (`Controller.UnPossess` (`GameplayStatics.GetPlayerController` 0))
  (bind _returnvalue (`GameplayStatics.GetActorOfClass` "/Game/UI/BP_MainHUD.BP_MainHUD_C"))
  (`/Game/UI/BP_MainHUD.ShowDeathScreen` _returnvalue)
  (`GameplayStatics.PlaySoundAtLocation` "/Game/Audio/MainCharacter/171050__amatvejuk721__death-breath_-_DEATH_MAIN_CHAR.171050__amatvejuk721__death-breath_-_DEATH_MAIN_CHAR" (0.0 0.0 0.0) (struct) 1.0 1.0 0.0 null null null))

(event `BossHasDied`
  ;[1 1 1] Manage boss death
  (bind _outactors (`GameplayStatics.GetAllActorsOfClass` "/Game/Blueprints/Enemies/BP_Enemy.BP_Enemy_C"))
  (for _array_element _outactors
    (`self.K2_DestroyActor` _array_element))
  (`Controller.UnPossess` (`GameplayStatics.GetPlayerController` 0))
  (bind _returnvalue (`GameplayStatics.GetActorOfClass` "/Game/UI/BP_MainHUD.BP_MainHUD_C"))
  (`/Game/UI/BP_MainHUD.ShowWinScreen` _returnvalue)
  (`KismetSystemLibrary.Delay` 15.0)
  (`GameplayStatics.OpenLevel` "StartScreen"))

(event `self.Pit Area.OnComponentBeginOverlap`
  (params (OverlappedComponent :type "PrimitiveComponent Object Reference") (OtherActor :type "Actor Object Reference") (OtherComp :type "PrimitiveComponent Object Reference") (OtherBodyIndex :type Integer) (bFromSweep :type Boolean) (SweepResult :type "HitResult Structure (by ref)"))
  (cast `/Game/Blueprints/Characters/BP_MainCharacter` OtherActor))

(event `InputAction|PauseMenu` :paused true
  (params (Key :type "Key Structure"))
  ;[1 1 1] Show Pause Menu
  (:`Pressed`
    (bind _returnvalue (`GameplayStatics.GetActorOfClass` "/Game/UI/BP_MainHUD.BP_MainHUD_C"))
    (`/Game/UI/BP_MainHUD.ShowPauseMenu` _returnvalue)
    (`GameplayStatics.SetGamePaused` true)))

(event `self.StartAreaMainChar.OnComponentBeginOverlap`
  (params (OverlappedComponent :type "PrimitiveComponent Object Reference") (OtherActor :type "Actor Object Reference") (OtherComp :type "PrimitiveComponent Object Reference") (OtherBodyIndex :type Integer) (bFromSweep :type Boolean) (SweepResult :type "HitResult Structure (by ref)"))
  ;[1 1 1] Show message to press TAB
  (bind _asbp_main_character (cast `/Game/Blueprints/Characters/BP_MainCharacter` OtherActor))
  (`/Engine/EditorBlueprintResources/StandardMacros.DoOnce` false
    (:`Completed`
      (`/Game/Blueprints/Characters/BP_MainCharacter.ShowMessagesText` _asbp_main_character "Press TAB to project  \nonto Axon")
      (`KismetSystemLibrary.Delay` (`self.MessageTime`))
      (bind _returnvalue (`GameplayStatics.GetActorOfClass` "/Game/Blueprints/Characters/BP_MainCharacter.BP_MainCharacter_C"))
      (`/Game/Blueprints/Characters/BP_MainCharacter.ClearMessagesText` _returnvalue))))

(event `self.StartAreaMainChar.OnComponentEndOverlap`
  (params (OverlappedComponent :type "PrimitiveComponent Object Reference") (OtherActor :type "Actor Object Reference") (OtherComp :type "PrimitiveComponent Object Reference") (OtherBodyIndex :type Integer))
  ;[1 1 1] Show message to press TAB
)

(event `self.GrabBoxAreaSecondChar.OnComponentBeginOverlap`
  (params (OverlappedComponent :type "PrimitiveComponent Object Reference") (OtherActor :type "Actor Object Reference") (OtherComp :type "PrimitiveComponent Object Reference") (OtherBodyIndex :type Integer) (bFromSweep :type Boolean) (SweepResult :type "HitResult Structure (by ref)"))
  ;[1 1 1] Show LEFT MOUSE grab
  (bind _asbp_secondary_character (cast `/Game/Blueprints/Characters/BP_SecondaryCharacter` OtherActor))
  (`/Engine/EditorBlueprintResources/StandardMacros.DoOnce` false
    (:`Completed`
      (`/Game/Blueprints/Characters/BP_SecondaryCharacter.ShowMessagesText` _asbp_secondary_character "LEFT MOUSE to grasp objects")
      (`KismetSystemLibrary.Delay` (- (`self.MessageTime`) 6.0))
      (bind _returnvalue (`GameplayStatics.GetActorOfClass` "/Game/Blueprints/Characters/BP_SecondaryCharacter.BP_SecondaryCharacter_C"))
      (`/Game/Blueprints/Characters/BP_SecondaryCharacter.ClearMessagesText` _returnvalue))))

(event `self.GrabBoxAreaSecondChar.OnComponentEndOverlap`
  (params (OverlappedComponent :type "PrimitiveComponent Object Reference") (OtherActor :type "Actor Object Reference") (OtherComp :type "PrimitiveComponent Object Reference") (OtherBodyIndex :type Integer))
  ;[1 1 1] Show LEFT MOUSE grab
)

(event `self.ReleaseBoxAreaSecondChar.OnComponentBeginOverlap`
  (params (OverlappedComponent :type "PrimitiveComponent Object Reference") (OtherActor :type "Actor Object Reference") (OtherComp :type "PrimitiveComponent Object Reference") (OtherBodyIndex :type Integer) (bFromSweep :type Boolean) (SweepResult :type "HitResult Structure (by ref)"))
  ;[1 1 1] Show RELEASE or THROW messages
  (bind _asbp_secondary_character (cast `/Game/Blueprints/Characters/BP_SecondaryCharacter` OtherActor))
  (`/Engine/EditorBlueprintResources/StandardMacros.DoOnce` false
    (:`Completed`
      (`/Game/Blueprints/Characters/BP_SecondaryCharacter.ShowMessagesText` _asbp_secondary_character "LEFT MOUSE to throw objects \nRIGHT MOUSE to release")
      (`KismetSystemLibrary.Delay` (- (`self.MessageTime`) 6.0))
      (bind _returnvalue (`GameplayStatics.GetActorOfClass` "/Game/Blueprints/Characters/BP_SecondaryCharacter.BP_SecondaryCharacter_C"))
      (`/Game/Blueprints/Characters/BP_SecondaryCharacter.ClearMessagesText` _returnvalue))))

(event `self.ReleaseBoxAreaSecondChar.OnComponentEndOverlap`
  (params (OverlappedComponent :type "PrimitiveComponent Object Reference") (OtherActor :type "Actor Object Reference") (OtherComp :type "PrimitiveComponent Object Reference") (OtherBodyIndex :type Integer))
  ;[1 1 1] Show RELEASE or THROW messages
)

(event `self.ElectricButtonAreaMainChar.OnComponentBeginOverlap`
  (params (OverlappedComponent :type "PrimitiveComponent Object Reference") (OtherActor :type "Actor Object Reference") (OtherComp :type "PrimitiveComponent Object Reference") (OtherBodyIndex :type Integer) (bFromSweep :type Boolean) (SweepResult :type "HitResult Structure (by ref)"))
  ;[1 1 1] Show message to activate buttons and bombs
  (bind _asbp_main_character (cast `/Game/Blueprints/Characters/BP_MainCharacter` OtherActor))
  (`/Engine/EditorBlueprintResources/StandardMacros.DoOnce` false
    (:`Completed`
      (`/Game/Blueprints/Characters/BP_MainCharacter.ShowMessagesText` _asbp_main_character "Electromechanical pulses  \ncan send synaptic \nsignals to interruptors and bombs")
      (`KismetSystemLibrary.Delay` (`self.MessageTime`))
      (bind _returnvalue (`GameplayStatics.GetActorOfClass` "/Game/Blueprints/Characters/BP_MainCharacter.BP_MainCharacter_C"))
      (`/Game/Blueprints/Characters/BP_MainCharacter.ClearMessagesText` _returnvalue))))

(event `self.ElectricButtonAreaMainChar.OnComponentEndOverlap`
  (params (OverlappedComponent :type "PrimitiveComponent Object Reference") (OtherActor :type "Actor Object Reference") (OtherComp :type "PrimitiveComponent Object Reference") (OtherBodyIndex :type Integer))
  ;[1 1 1] Show message to activate buttons and bombs
)

(event `self.EnemiesAreaMainChar.OnComponentBeginOverlap`
  (params (OverlappedComponent :type "PrimitiveComponent Object Reference") (OtherActor :type "Actor Object Reference") (OtherComp :type "PrimitiveComponent Object Reference") (OtherBodyIndex :type Integer) (bFromSweep :type Boolean) (SweepResult :type "HitResult Structure (by ref)"))
  ;[1 1 1] Show SHOOT message
  (bind _asbp_main_character (cast `/Game/Blueprints/Characters/BP_MainCharacter` OtherActor))
  (`/Engine/EditorBlueprintResources/StandardMacros.DoOnce` false
    (:`Completed`
      (`/Game/Blueprints/Characters/BP_MainCharacter.ShowMessagesText` _asbp_main_character "Generate electrochemical pulses \nwith LEFT MOUSE")
      (`KismetSystemLibrary.Delay` (`self.MessageTime`))
      (bind _returnvalue (`GameplayStatics.GetActorOfClass` "/Game/Blueprints/Characters/BP_MainCharacter.BP_MainCharacter_C"))
      (`/Game/Blueprints/Characters/BP_MainCharacter.ClearMessagesText` _returnvalue))))

(event `self.EnemiesAreaMainChar.OnComponentEndOverlap`
  (params (OverlappedComponent :type "PrimitiveComponent Object Reference") (OtherActor :type "Actor Object Reference") (OtherComp :type "PrimitiveComponent Object Reference") (OtherBodyIndex :type Integer))
  ;[1 1 1] Show SHOOT message
)

(event `ShowMessageSecondCharDead`
  (bind _returnvalue (`GameplayStatics.GetActorOfClass` "/Game/Blueprints/Characters/BP_MainCharacter.BP_MainCharacter_C"))
  (`/Game/Blueprints/Characters/BP_MainCharacter.ShowMessagesText` _returnvalue "When Axon is inhibited,  \nstress increases. \nRIGHT MOUSE to re-excite Axon")
  (`KismetSystemLibrary.Delay` (`self.MessageTime`))
  (`/Game/Blueprints/Characters/BP_MainCharacter.ClearMessagesText` _returnvalue))

(event `ShowMessageRevival`
  (bind _returnvalue (`GameplayStatics.GetActorOfClass` "/Game/Blueprints/Characters/BP_SecondaryCharacter.BP_SecondaryCharacter_C"))
  (`/Game/Blueprints/Characters/BP_SecondaryCharacter.ShowMessagesText` _returnvalue "Axon is immune for a brief moment \nafter being re-excited")
  (`KismetSystemLibrary.Delay` (`self.MessageTime`))
  (`/Game/Blueprints/Characters/BP_SecondaryCharacter.ClearMessagesText` _returnvalue))

(event `self.ChangeBackAreaSecondChar.OnComponentBeginOverlap`
  (params (OverlappedComponent :type "PrimitiveComponent Object Reference") (OtherActor :type "Actor Object Reference") (OtherComp :type "PrimitiveComponent Object Reference") (OtherBodyIndex :type Integer) (bFromSweep :type Boolean) (SweepResult :type "HitResult Structure (by ref)"))
  ;[1 1 1] Change back to Dr Ranvier message
  (bind _asbp_secondary_character (cast `/Game/Blueprints/Characters/BP_SecondaryCharacter` OtherActor))
  (`/Engine/EditorBlueprintResources/StandardMacros.DoOnce` false
    (:`Completed`
      (`/Game/Blueprints/Characters/BP_SecondaryCharacter.ShowMessagesText` _asbp_secondary_character "Press TAB to help Dr. Ranvier  \nget out of the cage")
      (`KismetSystemLibrary.Delay` (`self.MessageTime`))
      (bind _returnvalue (`GameplayStatics.GetActorOfClass` "/Game/Blueprints/Characters/BP_SecondaryCharacter.BP_SecondaryCharacter_C"))
      (`/Game/Blueprints/Characters/BP_SecondaryCharacter.ClearMessagesText` _asbp_secondary_character)
      (`/Game/Blueprints/Characters/BP_SecondaryCharacter.ClearMessagesText` _returnvalue))))

(event `self.BossAreaMainChar.OnComponentBeginOverlap`
  (params (OverlappedComponent :type "PrimitiveComponent Object Reference") (OtherActor :type "Actor Object Reference") (OtherComp :type "PrimitiveComponent Object Reference") (OtherBodyIndex :type Integer) (bFromSweep :type Boolean) (SweepResult :type "HitResult Structure (by ref)"))
  ;[1 1 1] Activate Bombs
  (bind _asbp_main_character (cast `/Game/Blueprints/Characters/BP_MainCharacter` OtherActor))
  (`/Engine/EditorBlueprintResources/StandardMacros.DoOnce` false
    (:`Completed`
      (`/Game/Blueprints/Characters/BP_MainCharacter.ShowMessagesText` _asbp_main_character "Neuroepithelial cysts are  \nvulnerable to explosions  \nin their blind spot")
      (`KismetSystemLibrary.Delay` (`self.MessageTime`))
      (bind _returnvalue (`GameplayStatics.GetActorOfClass` "/Game/Blueprints/Characters/BP_MainCharacter.BP_MainCharacter_C"))
      (`/Game/Blueprints/Characters/BP_MainCharacter.ClearMessagesText` _returnvalue))))

(event `self.BossAreaSecondChar.OnComponentBeginOverlap`
  (params (OverlappedComponent :type "PrimitiveComponent Object Reference") (OtherActor :type "Actor Object Reference") (OtherComp :type "PrimitiveComponent Object Reference") (OtherBodyIndex :type Integer) (bFromSweep :type Boolean) (SweepResult :type "HitResult Structure (by ref)"))
  (bind _asbp_secondary_character (cast `/Game/Blueprints/Characters/BP_SecondaryCharacter` OtherActor))
  (`/Engine/EditorBlueprintResources/StandardMacros.DoOnce` false
    (:`Completed`
      (`KismetSystemLibrary.Delay` 30.0)
      (`/Game/Blueprints/Characters/BP_SecondaryCharacter.ShowMessagesText` _asbp_secondary_character "Dr. Ranvier must activate \nthe magnetic bombs generator")
      (`KismetSystemLibrary.Delay` (`self.MessageTime`))
      (bind _returnvalue (`GameplayStatics.GetActorOfClass` "/Game/Blueprints/Characters/BP_SecondaryCharacter.BP_SecondaryCharacter_C"))
      (`/Game/Blueprints/Characters/BP_SecondaryCharacter.ClearMessagesText` _returnvalue))))

(event `EnemyHasDied`
  (params (EnemyDead :type "/Game/Blueprints/Enemies/BP_Enemy Object Reference"))
  (if (`PrimitiveComponent.IsOverlappingActor` (`self.Pit Area`) EnemyDead)
    (bind _result (`/Engine/EditorBlueprintResources/StandardMacros.IncrementInt` (`self.Integer`))
      (:`  `
        (if (>= _result 4)
          _)))))

(fn `UserConstructionScript`)