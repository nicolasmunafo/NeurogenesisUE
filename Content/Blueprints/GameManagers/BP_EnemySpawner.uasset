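; BP_EnemySpawner is a manager that spawns groups of patrolling BP_Enemy AI and replenishes them as they leave its area.
; SpawnEnemies places each enemy at a random actor from SpawningPointsArray, runs BP_EnemyBTree on it and assigns PatrolWaypoints.
; EnemiesArea end-overlap events decrement the live count and trigger a new wave at zero.
; BeginPlay is empty, so this graph never starts the first wave itself.
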(event `self.ReceiveBeginPlay`)

(event `self.ReceiveTick`
  (params (DeltaSeconds :type "Float (single-precision)")))

(event `Spawn Enemies`
  ;[1 1 1] Spawn enemies with a random location from SpawningPointsArray according to the PatrolWaypoints array
  (for _ (range 1 (+ (`self.EnemiesToSpawnNum`) 1))
    (bind _spawnlocation (`self.GetSpawnLocation`))
    (bind _returnvalue (`AIBlueprintHelperLibrary.SpawnAIFromClass` "/Game/Blueprints/Enemies/BP_Enemy.BP_Enemy_C" "/Game/Blueprints/Enemies/BP_EnemyBTree.BP_EnemyBTree" _spawnlocation (struct) false null))
    (bind _asbp_enemy (cast `/Game/Blueprints/Enemies/BP_Enemy` _returnvalue))
    (`/Game/Blueprints/Enemies/BP_Enemy.AssignPatrolWaypoints` _asbp_enemy (`self.PatrolWaypoints`)))
  (set `self.CurrentEnemies` (`self.EnemiesToSpawnNum`)))

(event `self.EnemiesArea.OnComponentEndOverlap`
  (params (OverlappedComponent :type "PrimitiveComponent Object Reference") (OtherActor :type "Actor Object Reference") (OtherComp :type "PrimitiveComponent Object Reference") (OtherBodyIndex :type Integer))
  (bind _currentenemies (`self.CurrentEnemies`))
  ;[1 1 1] When an enemy leaves the area, it decrements the counter and if there are 0 enemies, it spawns again
  (cast `/Game/Blueprints/Enemies/BP_Enemy` OtherActor)
  (`/Engine/EditorBlueprintResources/StandardMacros.DecrementInt` _currentenemies
    (:`  `
      (if (<= _currentenemies 0)
        (`self.Spawn Enemies`)))))

(fn `GetSpawnLocation`
  (returns (SpawnLocation :type "Vector Structure"))
  (bind _spawningpointsarray (`self.SpawningPointsArray`))
  (return (`self.K2_GetActorLocation` (`|GetArrayItem` _spawningpointsarray (`KismetMathLibrary.RandomIntegerInRange` 0 (`KismetArrayLibrary.Array_LastIndex` _spawningpointsarray))))))

(fn `UserConstructionScript`)