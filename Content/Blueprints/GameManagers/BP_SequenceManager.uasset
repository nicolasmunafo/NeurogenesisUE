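; BP_SequenceManager is a manager actor for a level's opening cinematic and the start of the main HUD.
; On BeginPlay, outside start levels, it either creates a player for StartSequence or calls BeginUI on BP_MainHUD and sets game-only input.
; The Play and OnFinished binding nodes are unconnected, so the sequence branch never plays or reaches the UI step.
; The custom StartSequence event is empty.
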(event `StartSequence`)

(event `self.ReceiveBeginPlay`
  ;[1 1 1] Play sequence and show basic UI unless is start level is TRUE
  (if (`self.isStartLevel`)
    _
    (elif (`self.showStartSequence`)
      (bind (_outactor _returnvalue) (`LevelSequencePlayer.CreateLevelSequencePlayer` "/Game/Sequences/StartSequence.StartSequence"))
      (else
        (bind _returnvalue_2 (`GameplayStatics.GetActorOfClass` "/Game/UI/BP_MainHUD.BP_MainHUD_C" :!label _label))
        (`/Game/UI/BP_MainHUD.BeginUI` _returnvalue_2)
        (`WidgetBlueprintLibrary.SetInputMode_GameOnly` (`GameplayStatics.GetPlayerController` 0))))))

(event `OnFinished_Event_0`
  ;[1 1 1] Play sequence and show basic UI unless is start level is TRUE
  (goto _label))

(fn `UserConstructionScript`)