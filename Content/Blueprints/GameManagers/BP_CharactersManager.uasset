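; Manager actor that switches player control between the main and secondary characters.
; On BeginPlay it finds both characters by class, and the ChangeCharacter input makes the player controller possess the other pawn, tracking which is current.
; Switching by input is blocked while the secondary is flagged dead; BlockToMainCharacter sets that flag, returning control to the main if needed, and ReviveSecondCharacter clears it and toggles control.
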(event `self.ReceiveBeginPlay`
  (`self.Initialization`))

(event `InputAction|ChangeCharacter`
  (params (Key :type "Key Structure"))
  (:`Pressed`
    (if (not (`self.IsSecondCharacterDead`))
      (`self.ChangeCharacter`))))

(event `BlockToMainCharacter`
  (if (== (`self.CurrentCharacter`) 2)
    (`self.ChangeCharacter`) ; If the current character is 2, change to 1 and \nset second character status to "dead"
  )
  (set `self.IsSecondCharacterDead` true) ; In both cases, the second character is dead
)

(event `ReviveSecondCharacter`
  (set `self.IsSecondCharacterDead` false)
  (`self.ChangeCharacter`))

(fn `ChangeCharacter`
  (bind _returnvalue (`GameplayStatics.GetPlayerController` 0))
  (if (== (`self.MainChar`) (`GameplayStatics.GetPlayerPawn` 0))
    (`Controller.Possess` _returnvalue (`self.SecondaryCharacter`))
    (set `self.CurrentCharacter` 2)
    (else
      (`Controller.Possess` _returnvalue (`self.MainChar`))
      (set `self.CurrentCharacter` 1))))

(fn `GetCurrentCharacter`
  (returns (NewParam :type Integer))
  (return (`self.CurrentCharacter`)))

(fn `Initialization`
  (bind _returnvalue (`GameplayStatics.GetActorOfClass` "/Game/Blueprints/Characters/BP_MainCharacter.BP_MainCharacter_C"))
  (set `self.MainChar` _returnvalue)
  (bind _returnvalue_2 (`GameplayStatics.GetActorOfClass` "/Game/Blueprints/Characters/BP_SecondaryCharacter.BP_SecondaryCharacter_C"))
  (set `self.SecondaryCharacter` _returnvalue_2)
  (set `self.CurrentCharacter` 1))

(fn `UserConstructionScript`)