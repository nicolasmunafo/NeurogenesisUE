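; Grabbable sticky bomb that attaches to surfaces and can be shot to damage the boss.
; On sphere hit with a "Stickable" component, it snaps to the impact point, attaches to that actor and notifies BP_Boss if hit.
; When shot while attached to the boss, it damages the boss's life component through its damage component.
; It then alerts boss and bomb spawner, destroys itself and plays explosion effects.
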(event `self.ReceiveTick`
  (params (DeltaSeconds :type "Float (single-precision)")))

(event `self.Sphere.OnComponentHit`
  (params (HitComponent :type "PrimitiveComponent Object Reference") (OtherActor :type "Actor Object Reference") (OtherComp :type "PrimitiveComponent Object Reference") (NormalImpulse :type "Vector Structure") (Hit :type "HitResult Structure (by ref)"))
  ;[1 1 1] If the sticky bomb hits an object tagged as "Stickable" it will stick at the location
  (if (`ActorComponent.ComponentHasTag` OtherComp "Stickable")
    (`self.K2_SetActorLocation` (`.ImpactPoint` (`GameplayStatics.BreakHitResult` Hit)))
    (`self.K2_AttachToActor` OtherActor "None" "KeepWorld" "KeepWorld" "KeepWorld")
    (bind _asbp_boss (cast `/Game/Blueprints/Boss/BP_Boss` OtherActor))
    (`/Game/Blueprints/Boss/BP_Boss.GotStickyBomb` _asbp_boss)))

(event `/Game/Blueprints/BP_IShootableActor.GetShotByCharacter`
  (params (Character :type "/Game/Blueprints/Characters/BP_MainCharacter Object Reference"))
  (bind _returnvalue (`self.K2_GetActorLocation`))
  (bind _returnvalue_2 (`self.GetAttachParentActor`))
  ;[1 1 1] When the character shoots the bomb, it has to damage the boss
  (`/Engine/EditorBlueprintResources/StandardMacros.IsValid` _returnvalue_2 ; Only explode if it has a parent
    (:`Is Valid`
      (bind _asbp_boss (cast `/Game/Blueprints/Boss/BP_Boss` _returnvalue_2))
      (`/Game/Blueprints/Components/BP_DamageComponent.Damage` (`self.BP_DamageComponent`) (`self.GetComponentByClass` _returnvalue_2 "/Game/Blueprints/Components/BP_LifeComponent.BP_LifeComponent_C"))
      (`/Game/Blueprints/Boss/BP_Boss.BombHasExploded` _asbp_boss)
      (bind _returnvalue_3 (`GameplayStatics.GetActorOfClass` "/Game/Blueprints/Switches/BP_BombsSpawner.BP_BombsSpawner_C"))
      (`/Game/Blueprints/Switches/BP_BombsSpawner.BombHasExploded` _returnvalue_3)
      (`self.K2_DestroyActor`)
      (`GameplayStatics.SpawnEmitterAtLocation` "/Game/StarterContent/Particles/P_Explosion.P_Explosion" _returnvalue (struct) (3.0 3.0 3.0))
      (`GameplayStatics.PlaySoundAtLocation` "/Game/StarterContent/Audio/Explosion01.Explosion01" _returnvalue (struct) 3.0 1.0 0.0 "/Game/Audio/SoundAttenuationBoss.SoundAttenuationBoss" null null))))

(fn `UserConstructionScript`)