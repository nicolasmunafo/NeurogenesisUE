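; Pressure button that opens an electric door while a BP_GrabbableBox rests on it and closes it when the box leaves.
; Collision overlaps sink or raise the button mesh and drive separate open and close timelines, each stopping the other and lerping from the door's current position toward marker locations.
; Opening also triggers a warning on all Widget_PIP widgets.
; ButtonIsPressed and ButtonIsReleased events change only the button state, without moving the door.
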(event `self.ReceiveBeginPlay`
  (set `self.DoorInitialPosition` (`SceneComponent.K2_GetComponentLocation` (`self.Door`))))

(event `OpenDoor`
  (`self.TriggerPIP`)
  (`|ExecutionSequence`
    (:`then_0`
      ;[1 1 1] Close the door and sets the button to inactive
      (bind (_direction _doorlerp) (`Timeline|Timeline_0` :!via `Stop` :!label _label)
        (:`Update`
          (`SceneComponent.K2_SetWorldLocation` (`self.Door`) (`KismetMathLibrary.VLerp` (`self.DoorCurrentPosition`) (`SceneComponent.K2_GetComponentLocation` (`self.InitialPosition`)) _doorlerp) false false))
        (:`Finished`
          (set `self.DoorInitialPosition` (`SceneComponent.K2_GetComponentLocation` (`self.Door`))))))
    (:`then_1`
      ;[1 1 1] Open the door with a timeline - Modify OpenDistance
      (set `self.DoorCurrentPosition` (`SceneComponent.K2_GetComponentLocation` (`self.Door`)))
      (bind (_direction_2 _doorlerp_2) (`Timeline|ElectricDoorTimeline` :!via `PlayFromStart` :!label _label_2)
        (:`Update`
          (`SceneComponent.K2_SetWorldLocation` (`self.Door`) (`KismetMathLibrary.VLerp` (`self.DoorCurrentPosition`) (`SceneComponent.K2_GetComponentLocation` (`self.EndPosition`)) _doorlerp_2) false false))
        (:`Finished`
          (set `self.DoorInitialPosition` (`SceneComponent.K2_GetComponentLocation` (`self.Door`))))))))

(event `CloseDoor`
  (`|ExecutionSequence`
    (:`then_0`
      (goto _label_2 :!via `Stop`))
    (:`then_1`
      ;[1 1 1] Close the door and sets the button to inactive
      (set `self.DoorCurrentPosition` (`SceneComponent.K2_GetComponentLocation` (`self.Door`)))
      (goto _label :!via `PlayFromStart`))))

(event `ButtonIsPressed`
  (if (not (`self.ButtonPressed`))
    (`self.PressButton`)
    (set `self.ButtonPressed` true)))

(event `ButtonIsReleased`
  (if (`self.ButtonPressed`)
    (`self.UnpressButton`)
    (set `self.ButtonPressed` false)))

(event `self.ButtonCollision.OnComponentBeginOverlap`
  (params (OverlappedComponent :type "PrimitiveComponent Object Reference") (OtherActor :type "Actor Object Reference") (OtherComp :type "PrimitiveComponent Object Reference") (OtherBodyIndex :type Integer) (bFromSweep :type Boolean) (SweepResult :type "HitResult Structure (by ref)"))
  (if (not (`self.ButtonPressed`))
    (cast `/Game/Blueprints/Grabbables/BP_GrabbableBox` OtherActor)
    (`self.PressButton`)
    (`self.OpenDoor`)
    (set `self.ButtonPressed` true)))

(event `self.ButtonCollision.OnComponentEndOverlap`
  (params (OverlappedComponent :type "PrimitiveComponent Object Reference") (OtherActor :type "Actor Object Reference") (OtherComp :type "PrimitiveComponent Object Reference") (OtherBodyIndex :type Integer))
  (if (`self.ButtonPressed`)
    (cast `/Game/Blueprints/Grabbables/BP_GrabbableBox` OtherActor)
    (`self.UnpressButton`)
    (`self.CloseDoor`)
    (set `self.ButtonPressed` false)))

(event `TriggerPIP`
  (bind _foundwidgets (`WidgetBlueprintLibrary.GetAllWidgetsOfClass` "/Game/UI/Widget_PIP.Widget_PIP_C"))
  (for _array_element _foundwidgets
    (`/Game/UI/Widget_PIP.TriggerWarning` _array_element)))

(fn `PressButton`
  (`SceneComponent.K2_AddWorldOffset` (`self.ButtonMesh`) (0.0 0.0 -20.0) false false)
  (`KismetSystemLibrary.PrintString` "Pressed"))

(fn `UnpressButton`
  (`SceneComponent.K2_AddWorldOffset` (`self.ButtonMesh`) (0.0 0.0 20.0) false false)
  (`KismetSystemLibrary.PrintString` "Unpressed"))

(fn `UserConstructionScript`)