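; BP_ElasticSwitch is a momentary switch that hides a wall while something overlaps its trigger and shows it again on release.
; The trigger's begin and end overlap events toggle the Wall component's visibility, set the Pressed flag and print it for debugging.
; Overlaps are not filtered by actor, and only visibility changes, with no collision change on the wall.
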(event `self.TriggerElasticSwitch.OnComponentBeginOverlap`
  (params (OverlappedComponent :type "PrimitiveComponent Object Reference") (OtherActor :type "Actor Object Reference") (OtherComp :type "PrimitiveComponent Object Reference") (OtherBodyIndex :type Integer) (bFromSweep :type Boolean) (SweepResult :type "HitResult Structure (by ref)"))
  (`SceneComponent.SetVisibility` (`self.Wall`) false false)
  (bind _output_get (set `self.Pressed` true))
  (`KismetSystemLibrary.PrintString` (`KismetStringLibrary.Conv_BoolToString` _output_get)))

(event `self.TriggerElasticSwitch.OnComponentEndOverlap`
  (params (OverlappedComponent :type "PrimitiveComponent Object Reference") (OtherActor :type "Actor Object Reference") (OtherComp :type "PrimitiveComponent Object Reference") (OtherBodyIndex :type Integer))
  (`SceneComponent.SetVisibility` (`self.Wall`) true false)
  (bind _output_get (set `self.Pressed` false))
  (`KismetSystemLibrary.PrintString` (`KismetStringLibrary.Conv_BoolToString` _output_get)))

(fn `UserConstructionScript`)