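; BP_BombsSpawner is a shootable switch that drops a sticky bomb into the scene, apparently for use against a boss.
; When shot with no bomb active, it plays a buzz, triggers the warning on picture-in-picture widgets and spawns BP_StickyBomb at a random SpawningPoints actor with a drop sound.
; A BombInScene flag blocks further spawns until BombHasExploded clears it.
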(event `TriggerPIP`
  (bind _foundwidgets (`WidgetBlueprintLibrary.GetAllWidgetsOfClass` "/Game/UI/Widget_PIP.Widget_PIP_C"))
  (for _array_element _foundwidgets
    (`/Game/UI/Widget_PIP.TriggerWarning` _array_element)))

(event `self.ReceiveBeginPlay`)

(event `/Game/Blueprints/BP_IShootableActor.GetShotByCharacter`
  (params (Character :type "/Game/Blueprints/Characters/BP_MainCharacter Object Reference"))
  ;[1 1 1] If the switch gets shot, it will spawn a bomb in a specific place
  (if (not (`self.BombInScene`))
    (`GameplayStatics.PlaySoundAtLocation` "/Game/Audio/Props/329778__visualasylum__electric-buzz-shock_-_ELECTRIC_BUTTON.329778__visualasylum__electric-buzz-shock_-_ELECTRIC_BUTTON" (`self.K2_GetActorLocation`) (struct) 1.0 1.0 0.0 "/Game/Audio/SoundAttenuationObjects.SoundAttenuationObjects" null null)
    (`self.SpawnBomb`)
    (set `self.BombInScene` true)))

(event `SpawnBomb`
  (bind _spawningpoints (`self.SpawningPoints`))
  ;[1 1 1] Spawn a bomb in one of the spawning points
  (`self.TriggerPIP`)
  (`|SpawnActorFromClass` "/Game/Blueprints/Grabbables/BP_StickyBomb.BP_StickyBomb_C" (`KismetMathLibrary.MakeTransform` (`self.K2_GetActorLocation` (`|GetArrayItem` _spawningpoints (`KismetMathLibrary.RandomIntegerInRange` 0 (`KismetArrayLibrary.Array_LastIndex` _spawningpoints))))) "Undefined" "OverrideRootScale" null null)
  (`GameplayStatics.PlaySoundAtLocation` "/Game/Audio/Props/388553__suzenako__bmb0_-_BOMB_DROP.388553__suzenako__bmb0_-_BOMB_DROP" (0.0 0.0 0.0) (struct) 1.0 1.0 0.0 null null null))

(event `BombHasExploded`
  ;[1 1 1] When the bomb gets shot in the boss, allow the character to spawn another bomb
  (set `self.BombInScene` false))

(fn `UserConstructionScript`)