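; BP_ElectricSwitch is a shootable switch that opens a referenced Door, then closes it again after OpenTime.
; GetShotbyCharacter uses an IsActive flag to ignore repeat shots until the door finishes closing.
; Two timelines lerp the door along world Y by plus or minus OpenDistance, re-caching its position as the next start point when each finishes.
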(event `self.ReceiveBeginPlay`
  (set `self.DoorInitialPosition` (`SceneComponent.K2_GetComponentLocation` (`self.Door`))))

(event `/Game/Blueprints/BP_IShootableActor.GetShotByCharacter`
  (params (Character :type "/Game/Blueprints/Characters/BP_MainCharacter Object Reference"))
  ;[1 1 1] If the switch gets shot, the door will open and after a time it will close
  (`KismetSystemLibrary.PrintString` "ouch")
  (if (not (`self.IsActive`))
    (set `self.IsActive` true)
    (`self.OpenDoor`)
    (`KismetSystemLibrary.Delay` (`self.OpenTime`))
    (`self.CloseDoor`)))

(event `OpenDoor`
  (bind _doorinitialposition (`self.DoorInitialPosition`))
  ;[1 1 1] Open the door with a timeline - Modify OpenDistance
  (bind (_direction _doorlerp) (`Timeline|ElectricDoorTimeline` :!via `PlayFromStart`)
    (:`Update`
      (`SceneComponent.K2_SetWorldLocation` (`self.Door`) (`KismetMathLibrary.VLerp` _doorinitialposition (`KismetMathLibrary.MakeVector` (.x _doorinitialposition) (+ (.y _doorinitialposition) (`self.OpenDistance`)) (.z _doorinitialposition)) _doorlerp) false false))
    (:`Finished`
      (set `self.DoorInitialPosition` (`SceneComponent.K2_GetComponentLocation` (`self.Door`))))))

(event `CloseDoor`
  (bind _doorinitialposition (`self.DoorInitialPosition`))
  ;[1 1 1] Close the door and sets the button to inactive
  (bind (_direction _doorlerp) (`Timeline|Timeline_0` :!via `PlayFromStart`)
    (:`Update`
      (`SceneComponent.K2_SetWorldLocation` (`self.Door`) (`KismetMathLibrary.VLerp` _doorinitialposition (`KismetMathLibrary.MakeVector` (.x _doorinitialposition) (- (.y _doorinitialposition) (`self.OpenDistance`)) (.z _doorinitialposition)) _doorlerp) false false))
    (:`Finished`
      (set `self.DoorInitialPosition` (`SceneComponent.K2_GetComponentLocation` (`self.Door`)))
      (set `self.IsActive` false))))

(fn `UserConstructionScript`)