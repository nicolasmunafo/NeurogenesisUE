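; BP_DoorClosedOnTrigger is a switch Blueprint that slides a door shut to an end position.
; CloseDoor captures the door's current location, then a timeline lerps it to EndPosition's world location.
; The CloseDoorTrigger overlap event is empty; its character-cast and DoOnce chain into CloseDoor is disconnected, so nothing in this graph closes the door.
; BeginPlay stores the initial door position, which is never read here.
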(event `self.ReceiveBeginPlay`
  (set `self.DoorInitialPosition` (`SceneComponent.K2_GetComponentLocation` (`self.Door`))))

(event `CloseDoor`
  ;[1 1 1] Close the door and sets the button to inactive
  (set `self.DoorCurrentPosition` (`SceneComponent.K2_GetComponentLocation` (`self.Door`)))
  (bind (_direction _doorlerp) (`Timeline|Timeline_0` :!via `PlayFromStart`)
    (:`Update`
      (`SceneComponent.K2_SetWorldLocation` (`self.Door`) (`KismetMathLibrary.VLerp` (`self.DoorCurrentPosition`) (`SceneComponent.K2_GetComponentLocation` (`self.EndPosition`)) _doorlerp) false false))))

(event `self.CloseDoorTrigger.OnComponentBeginOverlap`
  (params (OverlappedComponent :type "PrimitiveComponent Object Reference") (OtherActor :type "Actor Object Reference") (OtherComp :type "PrimitiveComponent Object Reference") (OtherBodyIndex :type Integer) (bFromSweep :type Boolean) (SweepResult :type "HitResult Structure (by ref)")))

(fn `UserConstructionScript`)